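; Speed boost item Blueprint that temporarily doubles the walk speed of the actor that activates it.
; On activation it stores that actor and sets its CharacterMovementComponent's MaxWalkSpeed to twice GetMaxSpeed.
; On expiry, if the actor is still valid, it sets MaxWalkSpeed to half the current GetMaxSpeed rather than restoring a saved value, then calls the parent's expiry logic.
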(event `self.OnActivated`
  (params (OtherActor :type "Actor Object Reference"))
  (bind _output_get (set `self.ActivateForPlayer` OtherActor))
  (bind _returnvalue (`self.GetComponentByClass` _output_get "/Script/Engine.CharacterMovementComponent"))
  (set `CharacterMovementComponent.MaxWalkSpeed` (* (`MovementComponent.GetMaxSpeed` _returnvalue) 2.0) _returnvalue))

(event `self.OnExpired`
  (bind _activateforplayer (`self.ActivateForPlayer`))
  (bind _returnvalue (`self.GetComponentByClass` _activateforplayer "/Script/Engine.CharacterMovementComponent"))
  (`/Engine/EditorBlueprintResources/StandardMacros.IsValid` _activateforplayer
    (:`Is Valid`
      (set `CharacterMovementComponent.MaxWalkSpeed` (/ (`MovementComponent.GetMaxSpeed` _returnvalue) 2.0) _returnvalue))
    (:`Is Not Valid`
      _))
  (`parent.OnExpired`))

(fn `UserConstructionScript`
  (`parent.UserConstructionScript`))