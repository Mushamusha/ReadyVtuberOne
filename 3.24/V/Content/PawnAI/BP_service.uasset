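; BP_service is a Behavior Tree service that picks the nearest hostile target for an AI pawn.
; Each tick it loops over the sight-known actors from the pawn's AIPerception component, keeping non-friendly ones with non-negative HealthComponent health.
; It writes the closest to a configurable blackboard key.
; BestTarget is not cleared between ticks, so the previous target can persist when none qualifies.
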(event `self.ReceiveTickAI`
  (params (OwnerController :type "AIController Object Reference") (ControlledPawn :type "Pawn Object Reference") (DeltaSeconds :type "Float (single-precision)"))
  (set `self.NearestDistance` 100000.0)
  (for _array_element (`AIPerceptionComponent.GetKnownPerceivedActors` (`Actor.GetComponentByClass` ControlledPawn "/Script/AIModule.AIPerceptionComponent") "/Script/AIModule.AISense_Sight")
    (if (and (not (`HealthComponent.IsFriendly` ControlledPawn _array_element)) (>= (`HealthComponent.Health` (`Actor.GetComponentByClass` _array_element "/Script/V.HealthComponent")) 0.0))
      (bind _returnvalue (`KismetMathLibrary.VSize` (- (`Actor.K2_GetActorLocation` ControlledPawn) (`Actor.K2_GetActorLocation` _array_element))))
      (if (< _returnvalue (`self.NearestDistance`))
        (set `self.NearestDistance` _returnvalue)
        (set `self.BestTarget` _array_element))))
  (`BTFunctionLibrary.SetBlackboardValueAsObject` (`self.BlackboardKey`) (`self.BestTarget`)))